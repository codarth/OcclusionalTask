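; Physics-driven player character that moves and jumps by pushing its static mesh, with mouse look, spring-arm zoom and an interact input that fires a referenced cannon.
; Both arms follow control pitch, carrying arrows that set each hand's physics-handle target.
; Hand inputs line-trace from the arrows to grab and release objects.
; Throw launches held objects along the arrows and blocks regrabbing: briefly for the right hand, permanently for the left.
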(event `self.ReceiveBeginPlay`
  (bind _returnvalue (`GameplayStatics.GetPlayerCameraManager` 0))
  (`EnhancedInputSubsystemInterface.AddMappingContext` (pcsubsystem `EnhancedInputLocalPlayerSubsystem` (`GameplayStatics.GetPlayerController` 0)) "/Game/_OcclusionalTask/Inputs/IC_Main.IC_Main" 0 (struct))
  (set `PlayerCameraManager.ViewPitchMin` -80.0 _returnvalue)
  (set `PlayerCameraManager.ViewPitchMax` 60.0 _returnvalue)
  (set `self.CanGrabRight` true)
  (set `self.CanGrabLeft` true))

(event `self.ReceiveTick`
  (params (DeltaSeconds :type "Float (single-precision)"))
  (bind (_returnvalue_roll _returnvalue_pitch) (`KismetMathLibrary.BreakRotator` (`self.GetControlRotation`)))
  (bind (_returnvalue_roll_2 _returnvalue_pitch_2 _returnvalue_yaw) (`KismetMathLibrary.BreakRotator` (`self.K2_GetActorRotation`)))
  (`SceneComponent.K2_SetWorldRotation` (`self.Arm_R`) (`KismetMathLibrary.MakeRotator` _returnvalue_roll_2 (+ _returnvalue_pitch -90.0) _returnvalue_yaw) false false)
  (`SceneComponent.K2_SetWorldRotation` (`self.Arm_L`) (`KismetMathLibrary.MakeRotator` _returnvalue_roll_2 (+ _returnvalue_pitch -90.0) _returnvalue_yaw) false false)
  (`PhysicsHandleComponent.SetTargetLocation` (`self.Hand_R`) (`SceneComponent.K2_GetComponentLocation` (`self.Arrow_R`)))
  (`PhysicsHandleComponent.SetTargetLocation` (`self.Hand_L`) (`SceneComponent.K2_GetComponentLocation` (`self.Arrow_L`))))

(event `EnhancedInput|/Game/_OcclusionalTask/Inputs/InputActions/IA_Look`
  (params (ActionValue :type "Vector2D Structure") (ElapsedSeconds :type "Float (double-precision)") (TriggeredSeconds :type "Float (double-precision)") (InputAction :type "InputAction Object Reference" :default "/Game/_OcclusionalTask/Inputs/InputActions/IA_Look.IA_Look"))
  (:`Triggered`
    (`self.AddControllerPitchInput` ActionValue_Y)
    (`self.AddControllerYawInput` ActionValue_X)))

(event `EnhancedInput|/Game/_OcclusionalTask/Inputs/InputActions/IA_Move`
  (params (ActionValue :type "Vector2D Structure") (ElapsedSeconds :type "Float (double-precision)") (TriggeredSeconds :type "Float (double-precision)") (InputAction :type "InputAction Object Reference" :default "/Game/_OcclusionalTask/Inputs/InputActions/IA_Move.IA_Move"))
  (bind (_returnvalue_roll _returnvalue_pitch _returnvalue_yaw) (`KismetMathLibrary.BreakRotator` (`self.GetControlRotation`)))
  (bind _returnvalue (`KismetMathLibrary.MakeRotator` 0.0 0.0 _returnvalue_yaw))
  (:`Triggered`
    (`PrimitiveComponent.AddForce` (`self.StaticMesh`) (* (`KismetMathLibrary.GetForwardVector` _returnvalue) ActionValue_Y (`self.MoveMultiplier`)) "None" false)
    (`PrimitiveComponent.AddForce` (`self.StaticMesh`) (* (`KismetMathLibrary.GetRightVector` _returnvalue) ActionValue_X (`self.MoveMultiplier`)) "None" false)))

(event `EnhancedInput|/Game/_OcclusionalTask/Inputs/InputActions/IA_RightHand`
  (params (ActionValue :type Boolean) (ElapsedSeconds :type "Float (double-precision)") (TriggeredSeconds :type "Float (double-precision)") (InputAction :type "InputAction Object Reference" :default "/Game/_OcclusionalTask/Inputs/InputActions/IA_RightHand.IA_RightHand"))
  (bind _arrow_r (`self.Arrow_R`))
  (bind _returnvalue (`SceneComponent.K2_GetComponentLocation` _arrow_r))
  (:`Triggered`
    (if (and (== (`PhysicsHandleComponent.GetGrabbedComponent` (`self.Hand_R`)) null) (`self.CanGrabRight`))
      (bind (_outhit _returnvalue_2) (`KismetSystemLibrary.LineTraceSingle` _returnvalue (+ _returnvalue (* (`SceneComponent.GetForwardVector` _arrow_r) (`self.PickupDistance`))) "TraceTypeQuery1"))
      (if _returnvalue_2
        (bind (_bblockinghit _binitialoverlap _time _distance _location _impactpoint _normal _impactnormal _physmat _hitactor _hitcomponent) (`GameplayStatics.BreakHitResult` _outhit))
        (`PhysicsHandleComponent.GrabComponentAtLocation` (`self.Hand_R`) _hitcomponent "None" _impactpoint))))
  (:`Completed`
    (`PhysicsHandleComponent.ReleaseComponent` (`self.Hand_R`))))

(event `EnhancedInput|/Game/_OcclusionalTask/Inputs/InputActions/IA_LeftHand`
  (params (ActionValue :type Boolean) (ElapsedSeconds :type "Float (double-precision)") (TriggeredSeconds :type "Float (double-precision)") (InputAction :type "InputAction Object Reference" :default "/Game/_OcclusionalTask/Inputs/InputActions/IA_LeftHand.IA_LeftHand"))
  (bind _arrow_l (`self.Arrow_L`))
  (bind _returnvalue (`SceneComponent.K2_GetComponentLocation` _arrow_l))
  (:`Triggered`
    (if (and (== (`PhysicsHandleComponent.GetGrabbedComponent` (`self.Hand_L`)) null) (`self.CanGrabLeft`))
      (bind (_outhit _returnvalue_2) (`KismetSystemLibrary.LineTraceSingle` _returnvalue (+ _returnvalue (* (`SceneComponent.GetForwardVector` _arrow_l) (`self.PickupDistance`))) "TraceTypeQuery1"))
      (if _returnvalue_2
        (bind (_bblockinghit _binitialoverlap _time _distance _location _impactpoint _normal _impactnormal _physmat _hitactor _hitcomponent) (`GameplayStatics.BreakHitResult` _outhit))
        (`PhysicsHandleComponent.GrabComponentAtLocation` (`self.Hand_L`) _hitcomponent "None" _impactpoint))))
  (:`Completed`
    (`PhysicsHandleComponent.ReleaseComponent` (`self.Hand_L`))))

(event `EnhancedInput|/Game/_OcclusionalTask/Inputs/InputActions/IA_Jump`
  (params (ActionValue :type Boolean) (ElapsedSeconds :type "Float (double-precision)") (TriggeredSeconds :type "Float (double-precision)") (InputAction :type "InputAction Object Reference" :default "/Game/_OcclusionalTask/Inputs/InputActions/IA_Jump.IA_Jump"))
  (bind _staticmesh (`self.StaticMesh`))
  (bind _returnvalue (`SceneComponent.K2_GetComponentLocation` _staticmesh))
  (:`Started`
    (bind (_outhit _returnvalue_2) (`KismetSystemLibrary.LineTraceSingle` _returnvalue (+ _returnvalue (* (`SceneComponent.GetUpVector` _staticmesh) -25.0)) "TraceTypeQuery1"))
    (if _returnvalue_2
      (`PrimitiveComponent.AddImpulse` (`self.StaticMesh`) (* (`KismetMathLibrary.Vector_Up`) (`self.JumpForce`)) "None" false))))

(event `EnhancedInput|/Game/_OcclusionalTask/Inputs/InputActions/IA_Interact`
  (params (ActionValue :type Boolean) (ElapsedSeconds :type "Float (double-precision)") (TriggeredSeconds :type "Float (double-precision)") (InputAction :type "InputAction Object Reference" :default "/Game/_OcclusionalTask/Inputs/InputActions/IA_Interact.IA_Interact"))
  (:`Started`
    (`/Game/_OcclusionalTask/Items/BP_Cannon.FireCannon` (`self.CannonREF`))))

(event `EnhancedInput|/Game/_OcclusionalTask/Inputs/InputActions/IA_Zoom`
  (params (ActionValue :type "Float (double-precision)") (ElapsedSeconds :type "Float (double-precision)") (TriggeredSeconds :type "Float (double-precision)") (InputAction :type "InputAction Object Reference" :default "/Game/_OcclusionalTask/Inputs/InputActions/IA_Zoom.IA_Zoom"))
  (bind _springarm (`self.SpringArm`))
  (:`Triggered`
    (set `SpringArmComponent.TargetArmLength` (`KismetMathLibrary.FClamp` (+ ActionValue (`SpringArmComponent.TargetArmLength` _springarm)) (`self.MinSpringArmLength`) (`self.MaxSpringArmLength`)) _springarm)))

(event `EnhancedInput|/Game/_OcclusionalTask/Inputs/InputActions/IA_Throw`
  (params (ActionValue :type Boolean) (ElapsedSeconds :type "Float (double-precision)") (TriggeredSeconds :type "Float (double-precision)") (InputAction :type "InputAction Object Reference" :default "/Game/_OcclusionalTask/Inputs/InputActions/IA_Throw.IA_Throw"))
  (bind _hand_l (`self.Hand_L`))
  (bind _hand_r (`self.Hand_R`))
  (:`Triggered`
    (`|ExecutionSequence`
      (:`then_0`
        (if (!= (`PhysicsHandleComponent.GetGrabbedComponent` (`self.Hand_R`)) null)
          (set `self.RightHandObjectREF` (`PhysicsHandleComponent.GetGrabbedComponent` _hand_r))
          (`PhysicsHandleComponent.ReleaseComponent` _hand_r)
          (`PrimitiveComponent.AddImpulse` (`self.RightHandObjectREF`) (* (`SceneComponent.GetForwardVector` (`self.Arrow_R`)) (`self.ThrowMultiplier`)) "None" false)
          (set `self.CanGrabRight` false)
          (`KismetSystemLibrary.Delay` 0.2)
          (set `self.CanGrabRight` true)))
      (:`then_1`
        (if (!= (`PhysicsHandleComponent.GetGrabbedComponent` (`self.Hand_L`)) null)
          (set `self.Left HandObjectREF` (`PhysicsHandleComponent.GetGrabbedComponent` _hand_l))
          (`PhysicsHandleComponent.ReleaseComponent` _hand_l)
          (`PrimitiveComponent.AddImpulse` (`self.Left HandObjectREF`) (* (`SceneComponent.GetForwardVector` (`self.Arrow_L`)) (`self.ThrowMultiplier`)) "None" false)
          (set `self.CanGrabLeft` false)
          (`KismetSystemLibrary.Delay` 0.2)
          (set `self.CanGrabLeft` false))))))

(fn `UserConstructionScript`)