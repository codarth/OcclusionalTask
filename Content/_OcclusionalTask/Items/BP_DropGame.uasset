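; BP_DropGame is a drop-style minigame that keeps a running score as items land in point zones.
; Paired overlap zones worth 10 to 50 points call SetScore, which accepts only BP_BaseItem actors and adds to a total that starts at zero on BeginPlay.
; Each change pushes the total to the UI_DropGameScore widget in ScoreWidget.
; A separate BallDeleter overlap volume destroys any BP_Ball that enters it.
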(event `self.ReceiveBeginPlay`
  (set `self.CurrentScore` 0)
  (`self.UpdateScoreUI`))

(event `self.Score_10_1.OnComponentBeginOverlap`
  (params (OverlappedComponent :type "PrimitiveComponent Object Reference") (OtherActor :type "Actor Object Reference") (OtherComp :type "PrimitiveComponent Object Reference") (OtherBodyIndex :type Integer) (bFromSweep :type Boolean) (SweepResult :type "HitResult Structure (by ref)"))
  (`self.SetScore` OtherActor 10))

(event `self.Score_10_2.OnComponentBeginOverlap`
  (params (OverlappedComponent :type "PrimitiveComponent Object Reference") (OtherActor :type "Actor Object Reference") (OtherComp :type "PrimitiveComponent Object Reference") (OtherBodyIndex :type Integer) (bFromSweep :type Boolean) (SweepResult :type "HitResult Structure (by ref)"))
  (`self.SetScore` OtherActor 10))

(event `self.Score_50_2.OnComponentBeginOverlap`
  (params (OverlappedComponent :type "PrimitiveComponent Object Reference") (OtherActor :type "Actor Object Reference") (OtherComp :type "PrimitiveComponent Object Reference") (OtherBodyIndex :type Integer) (bFromSweep :type Boolean) (SweepResult :type "HitResult Structure (by ref)"))
  (`self.SetScore` OtherActor 50))

(event `self.Score_50_1.OnComponentBeginOverlap`
  (params (OverlappedComponent :type "PrimitiveComponent Object Reference") (OtherActor :type "Actor Object Reference") (OtherComp :type "PrimitiveComponent Object Reference") (OtherBodyIndex :type Integer) (bFromSweep :type Boolean) (SweepResult :type "HitResult Structure (by ref)"))
  (`self.SetScore` OtherActor 50))

(event `self.Score_40_2.OnComponentBeginOverlap`
  (params (OverlappedComponent :type "PrimitiveComponent Object Reference") (OtherActor :type "Actor Object Reference") (OtherComp :type "PrimitiveComponent Object Reference") (OtherBodyIndex :type Integer) (bFromSweep :type Boolean) (SweepResult :type "HitResult Structure (by ref)"))
  (`self.SetScore` OtherActor 40))

(event `self.Score_40_1.OnComponentBeginOverlap`
  (params (OverlappedComponent :type "PrimitiveComponent Object Reference") (OtherActor :type "Actor Object Reference") (OtherComp :type "PrimitiveComponent Object Reference") (OtherBodyIndex :type Integer) (bFromSweep :type Boolean) (SweepResult :type "HitResult Structure (by ref)"))
  (`self.SetScore` OtherActor 40))

(event `self.Score_30_2.OnComponentBeginOverlap`
  (params (OverlappedComponent :type "PrimitiveComponent Object Reference") (OtherActor :type "Actor Object Reference") (OtherComp :type "PrimitiveComponent Object Reference") (OtherBodyIndex :type Integer) (bFromSweep :type Boolean) (SweepResult :type "HitResult Structure (by ref)"))
  (`self.SetScore` OtherActor 30))

(event `self.Score_30_1.OnComponentBeginOverlap`
  (params (OverlappedComponent :type "PrimitiveComponent Object Reference") (OtherActor :type "Actor Object Reference") (OtherComp :type "PrimitiveComponent Object Reference") (OtherBodyIndex :type Integer) (bFromSweep :type Boolean) (SweepResult :type "HitResult Structure (by ref)"))
  (`self.SetScore` OtherActor 30))

(event `self.Score_20_2.OnComponentBeginOverlap`
  (params (OverlappedComponent :type "PrimitiveComponent Object Reference") (OtherActor :type "Actor Object Reference") (OtherComp :type "PrimitiveComponent Object Reference") (OtherBodyIndex :type Integer) (bFromSweep :type Boolean) (SweepResult :type "HitResult Structure (by ref)"))
  (`self.SetScore` OtherActor 20))

(event `self.Score_20_1.OnComponentBeginOverlap`
  (params (OverlappedComponent :type "PrimitiveComponent Object Reference") (OtherActor :type "Actor Object Reference") (OtherComp :type "PrimitiveComponent Object Reference") (OtherBodyIndex :type Integer) (bFromSweep :type Boolean) (SweepResult :type "HitResult Structure (by ref)"))
  (`self.SetScore` OtherActor 20))

(event `self.BallDeleter.OnComponentBeginOverlap`
  (params (OverlappedComponent :type "PrimitiveComponent Object Reference") (OtherActor :type "Actor Object Reference") (OtherComp :type "PrimitiveComponent Object Reference") (OtherBodyIndex :type Integer) (bFromSweep :type Boolean) (SweepResult :type "HitResult Structure (by ref)"))
  (bind _asbp_ball (cast `/Game/_OcclusionalTask/Items/BP_Ball` OtherActor))
  (`self.K2_DestroyActor` _asbp_ball))

(fn `SetScore`
  (params (Object :type "Object Object Reference") (InScore :type Integer))
  (cast `/Game/_OcclusionalTask/Items/BP_BaseItem` Object)
  (set `self.CurrentScore` (+ (`self.CurrentScore`) InScore))
  (`self.UpdateScoreUI`))

(fn `UpdateScoreUI`
  (bind _asui_drop_game_score (cast `/Game/_OcclusionalTask/UI/UI_DropGameScore` (`WidgetComponent.GetWidget` (`self.ScoreWidget`))))
  (`/Game/_OcclusionalTask/UI/UI_DropGameScore.UpdateScore` _asui_drop_game_score (`self.CurrentScore`)))

(fn `UserConstructionScript`)