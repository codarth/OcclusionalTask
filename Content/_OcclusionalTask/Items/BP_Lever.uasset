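; BP_Lever is a lever actor that triggers physics on a linked BP_HideyBox when its handle flips.
; Every tick it converts the Handle's world rotation into actor space and reduces the pitch to a negative or non-negative state.
; When that state differs from LastState, it stores the new value and calls BeginPhysics on ObjectRef cast to BP_HideyBox, so flips in either direction trigger it.
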(event `self.ReceiveTick`
  (params (DeltaSeconds :type "Float (single-precision)"))
  (bind (_returnvalue_roll _returnvalue_pitch) (`KismetMathLibrary.BreakRotator` (`KismetMathLibrary.InverseTransformRotation` (`self.GetTransform`) (`SceneComponent.K2_GetComponentRotation` (`self.Handle`)))))
  (bind _returnvalue (< _returnvalue_pitch 0.0))
  (if (!= (`self.LastState`) _returnvalue)
    (set `self.LastState` _returnvalue)
    (bind _asbp_hidey_box (cast `/Game/_OcclusionalTask/Items/BP_HideyBox` (`self.ObjectRef`)))
    (`/Game/_OcclusionalTask/Items/BP_HideyBox.BeginPhysics` _asbp_hidey_box)))

(fn `UserConstructionScript`)