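; BP_Cannon is an interactable cannon that loads a BP_BaseItem as ammunition and launches it.
; An item entering LoadTrigger is hidden and attached to the barrel, with physics off and its mass saved.
; InteractRange registers the cannon with the player character and arms FireCannon, which restores the item and applies a forward impulse with a bang.
; The logic matching barrel rotation to AngleHandle is disconnected.
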(event `self.ReceiveTick`
  (params (DeltaSeconds :type "Float (single-precision)")))

(event `self.LoadTrigger.OnComponentBeginOverlap`
  (params (OverlappedComponent :type "PrimitiveComponent Object Reference") (OtherActor :type "Actor Object Reference") (OtherComp :type "PrimitiveComponent Object Reference") (OtherBodyIndex :type Integer) (bFromSweep :type Boolean) (SweepResult :type "HitResult Structure (by ref)"))
  (bind _cannonballref (`self.CannonBallREF`))
  (bind _staticmesh (`/Game/_OcclusionalTask/Items/BP_BaseItem.StaticMesh` (`self.CannonBallREF`)))
  (`self.CannonBallREF`
    (:`then`)
    (:`else`
      (bind _asbp_base_item (cast `/Game/_OcclusionalTask/Items/BP_BaseItem` OtherActor))
      (set `self.CannonBallREF` _asbp_base_item)
      (set `self.SavedMass` (`PrimitiveComponent.GetMass` _staticmesh))
      (`PrimitiveComponent.SetMassOverrideInKg` _staticmesh "None" 0.0 true)
      (`PrimitiveComponent.SetSimulatePhysics` _staticmesh false)
      (`SceneComponent.SetVisibility` _staticmesh false true)
      (`self.K2_SetActorLocation` _cannonballref (`SceneComponent.K2_GetComponentLocation` (`self.CannonBallLocation`)) false false)
      (`self.K2_AttachToComponent` _cannonballref (`self.Barrel`) "None" "KeepWorld" "KeepWorld" "KeepWorld" false)
      (set `self.IsLoaded` true))))

(event `self.InteractRange.OnComponentBeginOverlap`
  (params (OverlappedComponent :type "PrimitiveComponent Object Reference") (OtherActor :type "Actor Object Reference") (OtherComp :type "PrimitiveComponent Object Reference") (OtherBodyIndex :type Integer) (bFromSweep :type Boolean) (SweepResult :type "HitResult Structure (by ref)"))
  (bind _asbp_player_character (cast `/Game/_OcclusionalTask/Character/BP_PlayerCharacter` OtherActor))
  (set `self.IsReadyToFire` true)
  (set `/Game/_OcclusionalTask/Character/BP_PlayerCharacter.CannonREF` self _asbp_player_character))

(event `self.InteractRange.OnComponentEndOverlap`
  (params (OverlappedComponent :type "PrimitiveComponent Object Reference") (OtherActor :type "Actor Object Reference") (OtherComp :type "PrimitiveComponent Object Reference") (OtherBodyIndex :type Integer))
  (set `self.IsReadyToFire` false))

(event `FireCannon`
  (bind _staticmesh (`/Game/_OcclusionalTask/Items/BP_BaseItem.StaticMesh` (`self.CannonBallREF`)))
  (if (and (`self.IsReadyToFire`) (`self.IsLoaded`))
    (`self.CannonBallREF`
      (:`then`
        (`self.K2_DetachFromActor` (`self.CannonBallREF`) "KeepWorld" "KeepWorld" "KeepWorld")
        (`PrimitiveComponent.SetMassOverrideInKg` _staticmesh "None" (`self.SavedMass`) true)
        (`PrimitiveComponent.SetSimulatePhysics` _staticmesh true)
        (`SceneComponent.SetVisibility` _staticmesh true true)
        (`PrimitiveComponent.AddImpulse` (`/Game/_OcclusionalTask/Items/BP_BaseItem.StaticMesh` (`self.CannonBallREF`)) (* (`SceneComponent.GetForwardVector` (`self.CannonBallLocation`)) (`self.FireImpuleAmount`)) "None" false)
        (set `self.CannonBallREF` null)
        (set `self.IsLoaded` false)
        (`GameplayStatics.PlaySoundAtLocation` "/Game/_OcclusionalTask/Audio/BigBang.BigBang" (`SceneComponent.K2_GetComponentLocation` (`self.CannonBallLocation`)) (struct) 1.0 1.0 0.0 null null null null))
      (:`else`))))

(fn `UserConstructionScript`)